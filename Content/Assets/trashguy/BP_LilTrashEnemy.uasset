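; BP_LilTrashEnemy is an enemy character that chases the player when they come within range.
; Each Tick, a distance-only check compares the player pawn against DetectionRadius, with no line-of-sight test.
; In range it reissues AIMoveTo on the player every frame; otherwise it stops movement immediately.
; A direct-steering alternative, SimpleChasePlayer, exists but is never run.
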(event `self.ReceiveTick`
  (params (DeltaSeconds :type "Float (single-precision)"))
  (if (`self.bHasSpottedPlayer`)
    (`|AIMoveTo` self (0.0 0.0 0.0) (`GameplayStatics.GetPlayerPawn` 0))
    (else
      (`MovementComponent.StopMovementImmediately` (`self.CharacterMovement`)))))

(fn `bHasSpottedPlayer`
  (returns (Result :type Boolean))
  (`/Engine/EditorBlueprintResources/StandardMacros.IsValid` (`GameplayStatics.GetPlayerPawn` 0)
    (:`Is Valid`
      (return (<= (`KismetMathLibrary.VSize` (- (`self.K2_GetActorLocation` (`GameplayStatics.GetPlayerPawn` 0)) (`self.K2_GetActorLocation`))) (`self.DetectionRadius`))))
    (:`Is Not Valid`
      (return false))))

(fn `SimpleChasePlayer`
  (`/Engine/EditorBlueprintResources/StandardMacros.IsValid` (`GameplayStatics.GetPlayerCharacter` 0)
    (:`Is Valid`
      (`self.AddMovementInput` (`KismetMathLibrary.Normal` (- (`self.K2_GetActorLocation` (`GameplayStatics.GetPlayerCharacter` 0)) (`self.K2_GetActorLocation`)))))))

(fn `UserConstructionScript`)