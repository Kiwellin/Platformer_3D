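; Collectible cube actor that reports its pickup to the player's UI and animates before disappearing.
; OnCollected notifies the ThirdPersonCharacter's CollectibleWidget that a cube was collected.
; PlayCollectAnimation runs the Anim timeline to drive the Pivot's uniform scale, then destroys the actor when it finishes.
; Neither event is triggered in this graph, and its own overlap handler is disabled.
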(event `self.OnCollected`
  (params (ThirdPersonCharacter :type "/Game/BPs/BP_ThirdPersonCharacter Object Reference"))
  (`/Game/UI/BPW_CollectibleInfo.OnCollectedCube` (`/Game/BPs/BP_ThirdPersonCharacter.CollectibleWidget` ThirdPersonCharacter)))

(event `self.PlayCollectAnimation`
  (bind (_direction _scale) (`Timeline|anim`)
    (:`Update`
      (`SceneComponent.SetRelativeScale3D` (`self.Pivot`) (* (1.0 1.0 1.0) _scale)))
    (:`Finished`
      (`self.K2_DestroyActor`))))

(fn `UserConstructionScript`
  (`parent.UserConstructionScript`))