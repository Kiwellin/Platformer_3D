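; Interactable door Blueprint that swings open and closed around a pivot component.
; Each Interact event alternates through a FlipFlop between playing and reversing the OpenDoor timeline.
; The timeline's Door track, scaled by HowMuchDoorOpen, sets the Pivot's relative yaw.
; Disconnected leftover logic for IsOpening and IsDoorOpen state tracking never runs, and the construction script only calls its parent.
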(event `self.Interact`
  (`/Engine/EditorBlueprintResources/StandardMacros.FlipFlop`
    (:`A`
      (bind (_direction _door) (`Timeline|open door` :!label _label)
        (:`Update`
          (`SceneComponent.K2_SetRelativeRotation` (`self.Pivot`) (`KismetMathLibrary.MakeRotator` 0.0 0.0 (* _door (`self.HowMuchDoorOpen`))) false false))))
    (:`B`
      (goto _label :!via `Reverse`))))

(fn `UserConstructionScript`
  (`parent.UserConstructionScript`))