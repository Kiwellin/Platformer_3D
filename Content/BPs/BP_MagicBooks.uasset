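; BP_MagicBooks is an actor that moves its Pivot between two positions when its Activate event is called.
; Activate sets the Timeline play rate from the Speed variable and plays it from the start.
; Each update sets the Pivot's relative transform, with its location interpolated from the Start component to the End component by the timeline track.
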(event `self.ReceiveBeginPlay`)

(event `Activate`
  (`TimelineComponent.SetPlayRate` (`self.Timeline`) (`self.Speed`))
  (bind (_direction _newtrack_1) (`Timeline|Timeline` :!via `PlayFromStart`)
    (:`Update`
      (`SceneComponent.K2_SetRelativeTransform` (`self.Pivot`) (`KismetMathLibrary.MakeTransform` (`KismetMathLibrary.VLerp` (`SceneComponent.RelativeLocation` (`self.start`)) (`SceneComponent.RelativeLocation` (`self.end`)) _newtrack_1)) false false))))

(fn `UserConstructionScript`)