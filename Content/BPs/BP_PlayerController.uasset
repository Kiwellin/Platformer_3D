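; Player controller that routes Enhanced Input to the possessed BP_ThirdPersonCharacter, cached on possession.
; It adds the third-person mapping context on BeginPlay, then forwards camera, movement, sprint, interact, spell and emote actions to the character.
; Jump fires once per press through a DoOnce, saving velocity and toggling gravity scale until release.
; Fire and plant spells run only when the character's flags allow them.
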(event `self.ReceiveBeginPlay`
  (`EnhancedInputSubsystemInterface.AddMappingContext` (subsystem `EnhancedInputLocalPlayerSubsystem`) "/Game/Input/IMC_ThirdPerson.IMC_ThirdPerson" 0 (struct)))

(event `self.ReceivePossess`
  (params (PossessedPawn :type "Pawn Object Reference"))
  (bind _asbp_third_person_character (cast `/Game/BPs/BP_ThirdPersonCharacter` PossessedPawn))
  (set `self.Possessed Third Person Character` _asbp_third_person_character))

(event `EnhancedInput|/Game/Input/InputActions/IA_RotateCamera`
  (params (ActionValue :type "Vector2D Structure") (ElapsedSeconds :type "Float (double-precision)") (TriggeredSeconds :type "Float (double-precision)") (InputAction :type "InputAction Object Reference" :default "/Game/Input/InputActions/IA_RotateCamera.IA_RotateCamera"))
  (bind _possessed_third_person_character (`self.Possessed Third Person Character`))
  (:`Triggered`
    (`Pawn.AddControllerYawInput` _possessed_third_person_character ActionValue_X)
    (`Pawn.AddControllerPitchInput` _possessed_third_person_character ActionValue_Y)))

(event `EnhancedInput|/Game/Input/InputActions/IA_Jump`
  (params (ActionValue :type Boolean) (ElapsedSeconds :type "Float (double-precision)") (TriggeredSeconds :type "Float (double-precision)") (InputAction :type "InputAction Object Reference" :default "/Game/Input/InputActions/IA_Jump.IA_Jump"))
  (bind _possessed_third_person_character (`self.Possessed Third Person Character`))
  (:`Triggered`
    (if (`Character.CanJump` _possessed_third_person_character)
      (`/Engine/EditorBlueprintResources/StandardMacros.DoOnce` false :!label _label
        (:`Completed`
          (`Character.Jump` _possessed_third_person_character)
          (`/Game/BPs/BP_ThirdPersonCharacter.SaveLastVel` _possessed_third_person_character)
          (`/Game/BPs/BP_ThirdPersonCharacter.SetGravityScale` _possessed_third_person_character true)))))
  (:`Completed`
    (`/Game/BPs/BP_ThirdPersonCharacter.SetGravityScale` (`self.Possessed Third Person Character`) false)
    (goto _label :!via `Reset`)))

(event `EnhancedInput|/Game/Input/InputActions/IA_Move`
  (params (ActionValue :type "Vector2D Structure") (ElapsedSeconds :type "Float (double-precision)") (TriggeredSeconds :type "Float (double-precision)") (InputAction :type "InputAction Object Reference" :default "/Game/Input/InputActions/IA_Move.IA_Move"))
  (:`Triggered`
    (`/Game/BPs/BP_ThirdPersonCharacter.MoveInWorldDirection` (`self.Possessed Third Person Character`) (`KismetMathLibrary.MakeVector` ActionValue_X ActionValue_Y))))

(event `EnhancedInput|/Game/Input/InputActions/IA_Interact`
  (params (ActionValue :type Boolean) (ElapsedSeconds :type "Float (double-precision)") (TriggeredSeconds :type "Float (double-precision)") (InputAction :type "InputAction Object Reference" :default "/Game/Input/InputActions/IA_Interact.IA_Interact"))
  (:`Triggered`
    (`/Game/BPs/BP_ThirdPersonCharacter.TryInteract` (`self.Possessed Third Person Character`))))

(event `EnhancedInput|/Game/Input/InputActions/IA_Sprint`
  (params (ActionValue :type Boolean) (ElapsedSeconds :type "Float (double-precision)") (TriggeredSeconds :type "Float (double-precision)") (InputAction :type "InputAction Object Reference" :default "/Game/Input/InputActions/IA_Sprint.IA_Sprint"))
  (:`Started`
    (`/Game/BPs/BP_ThirdPersonCharacter.Sprint` (`self.Possessed Third Person Character`) ActionValue :!label _label_2))
  (:`Completed`
    (goto _label_2)))

(event `EnhancedInput|/Game/Input/InputActions/IA_SpellCast`
  (params (ActionValue :type Boolean) (ElapsedSeconds :type "Float (double-precision)") (TriggeredSeconds :type "Float (double-precision)") (InputAction :type "InputAction Object Reference" :default "/Game/Input/InputActions/IA_SpellCast.IA_SpellCast"))
  (:`Triggered`
    (`/Game/BPs/BP_ThirdPersonCharacter.CastSpell` (`self.Possessed Third Person Character`))))

(event `EnhancedInput|/Game/Input/InputActions/IA_FireSpell`
  (params (ActionValue :type Boolean) (ElapsedSeconds :type "Float (double-precision)") (TriggeredSeconds :type "Float (double-precision)") (InputAction :type "InputAction Object Reference" :default "/Game/Input/InputActions/IA_FireSpell.IA_FireSpell"))
  (bind _possessed_third_person_character (`self.Possessed Third Person Character`))
  (:`Triggered`
    (if (`/Game/BPs/BP_ThirdPersonCharacter.CanFireSpell` _possessed_third_person_character)
      (`/Game/BPs/BP_ThirdPersonCharacter.FireSpell` _possessed_third_person_character))))

(event `EnhancedInput|/Game/Input/InputActions/IA_PlantSpell`
  (params (ActionValue :type Boolean) (ElapsedSeconds :type "Float (double-precision)") (TriggeredSeconds :type "Float (double-precision)") (InputAction :type "InputAction Object Reference" :default "/Game/Input/InputActions/IA_PlantSpell.IA_PlantSpell"))
  (bind _possessed_third_person_character (`self.Possessed Third Person Character`))
  (:`Triggered`
    (if (`/Game/BPs/BP_ThirdPersonCharacter.CanPlantSpell` _possessed_third_person_character)
      (`/Game/BPs/BP_ThirdPersonCharacter.PlantSpell` _possessed_third_person_character))))

(event `EnhancedInput|/Game/Input/InputActions/IA_Emote`
  (params (ActionValue :type Boolean) (ElapsedSeconds :type "Float (double-precision)") (TriggeredSeconds :type "Float (double-precision)") (InputAction :type "InputAction Object Reference" :default "/Game/Input/InputActions/IA_Emote.IA_Emote"))
  (:`Triggered`
    (`AnimInstance.Montage_Play` (`SkeletalMeshComponent.GetAnimInstance` (`Character.Mesh` (`self.Possessed Third Person Character`))) "/Game/EpicCharacter/Animations/EpicCharacter_Celebrate_Montage.EpicCharacter_Celebrate_Montage" 1.0 "MontageLength" 0.0 true)))

(fn `UserConstructionScript`)