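; Interactable respawn point that registers itself as the player's respawn spot.
; On Interact, it casts player pawn 0 to BP_ThirdPersonCharacter and sets that character's MyRespawnPoint to itself.
; GetRespawnLocation supplies the world location and rotation of the RespawnPivot component as the respawn transform.
; The overlap event is empty, and disconnected leftover nodes for setting the respawn point or location never run.
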(event `self.ReceiveActorBeginOverlap`
  (params (OtherActor :type "Actor Object Reference")))

(event `self.Interact`
  (bind _asbp_third_person_character (cast `/Game/BPs/BP_ThirdPersonCharacter` (`GameplayStatics.GetPlayerPawn` 0)))
  (set `/Game/BPs/BP_ThirdPersonCharacter.MyRespawnPoint` self _asbp_third_person_character))

(fn `GetRespawnLocation`
  (returns (Location :type "Vector Structure") (Rotation :type "Rotator Structure"))
  (bind _respawnpivot (`self.RespawnPivot`))
  (return (`SceneComponent.K2_GetComponentLocation` _respawnpivot) (`SceneComponent.K2_GetComponentRotation` _respawnpivot)))

(fn `UserConstructionScript`)