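; BP_RuneStone is a rune stone actor that glows, rises and spins as the player approaches.
; BeginPlay creates a dynamic material instance on the stone mesh.
; Each Tick turns the player pawn's distance into a clamped 0–1 proximity factor that drives emission strength and float height directly.
; Yaw spin uses that factor squared, scaled by max speed and delta time, so rotation ramps up sharply up close.
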(event `self.ReceiveBeginPlay`
  (bind _returnvalue (`PrimitiveComponent.CreateDynamicMaterialInstance` (`self.RuneStone`) 0 null "None"))
  (set `self.Stone MID` _returnvalue))

(event `self.ReceiveTick`
  (params (DeltaSeconds :type "Float (single-precision)"))
  (bind _returnvalue (- 1.0 (`KismetMathLibrary.FClamp` (/ (`KismetMathLibrary.VSize` (- (`self.K2_GetActorLocation`) (`self.K2_GetActorLocation` (`GameplayStatics.GetPlayerPawn` 0)))) 1000.0))))
  (`MaterialInstanceDynamic.SetScalarParameterValue` (`self.Stone MID`) "EmissionStrength" _returnvalue)
  (`SceneComponent.K2_SetRelativeLocation` (`self.RuneStone`) (`KismetMathLibrary.MakeVector` 0.0 0.0 (* (`self.FloatHeight`) _returnvalue)) false false)
  (`SceneComponent.K2_AddRelativeRotation` (`self.RuneStone`) (`KismetMathLibrary.MakeRotator` 0.0 0.0 (* (* _returnvalue _returnvalue) (`self.Max Rotation Speed`) (`GameplayStatics.GetWorldDeltaSeconds`))) false false))

(fn `UserConstructionScript`)