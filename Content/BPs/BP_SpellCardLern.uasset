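; BP_SpellCardLern is an interactable spell card that brings up a spell card widget for the player to look at.
; Interact, on alternate calls via a FlipFlop, zeroes character velocity, switches to UI-only input, creates BP_SpellWidget once, plays its card animation and focuses its button.
; StopLooking restores game input and reverses the animation, but nothing in this graph's live paths calls it.
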(event `self.ReceiveBeginPlay`
  (`parent.ReceiveBeginPlay`)
  (bind _asbp_third_person_character (cast `/Game/BPs/BP_ThirdPersonCharacter` (`GameplayStatics.GetPlayerPawn` 0)))
  (set `self.TPCharacter` _asbp_third_person_character))

(event `self.Interact`
  (`/Engine/EditorBlueprintResources/StandardMacros.FlipFlop`
    (:`A`
      (`self.LookAtCard`))))

(event `LookAtCard`
  (bind _returnvalue (`GameplayStatics.GetPlayerController` 0))
  (set `MovementComponent.Velocity` (0.0 0.0 0.0) (`Character.CharacterMovement` (`self.TPCharacter`)))
  (`WidgetBlueprintLibrary.SetInputMode_UIOnlyEx` _returnvalue null "DoNotLock" true)
  (`self.SpellWidget`
    (:`then`
      _)
    (:`else`
      (bind _returnvalue_2 (`|CreateWidget` "/Game/UI/BP_SpellWidget.BP_SpellWidget_C" _returnvalue))
      (bind _output_get (set `self.SpellWidget` _returnvalue_2))
      (`UserWidget.AddToPlayerScreen` _output_get 0)))
  (`UserWidget.PlayAnimationForward` _output_get (`/Game/UI/BP_SpellWidget.MoveCardUpDown` _output_get) 1.0 false)
  (`KismetSystemLibrary.Delay` 0.2)
  (`Widget.SetFocus` (`/Game/UI/BP_SpellWidget.Button_50` _returnvalue_2)))

(event `StopLooking`
  (`WidgetBlueprintLibrary.SetInputMode_GameOnly` (`GameplayStatics.GetPlayerController` 0) true)
  (`UserWidget.PlayAnimationReverse` (stale `LookAtCard` _output_get) (`/Game/UI/BP_SpellWidget.MoveCardUpDown` (stale `LookAtCard` _output_get)) 1.0 false))

(fn `UserConstructionScript`
  (`parent.UserConstructionScript`))