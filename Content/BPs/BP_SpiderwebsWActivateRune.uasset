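; BP_SpiderwebsWActivateRune is a spiderweb actor that fades out and is removed when hit by a BP_FireSpell.
; BeginPlay creates a dynamic material instance on its Plane.
; A component hit from the fire spell calls Destroy, whose timeline drives the material's FadeAmount parameter, then destroys the actor.
; Despite the name, its BPSpellActivatedRune reference is unused, and a debug print remains in Destroy.
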(event `self.ReceiveBeginPlay`
  (bind _returnvalue (`PrimitiveComponent.CreateDynamicMaterialInstance` (`self.Plane`) 0 null "None"))
  (set `self.SpiderMID` _returnvalue))

(event `self.ReceiveTick`
  (params (DeltaSeconds :type "Float (single-precision)")))

(event `Destroy`
  (`KismetSystemLibrary.PrintString` "Hello")
  (bind (_direction _newtrack_0) (`Timeline|Timeline`)
    (:`Update`
      (`MaterialInstanceDynamic.SetScalarParameterValue` (`self.SpiderMID`) "FadeAmount" (* _newtrack_0 4.0)))
    (:`Finished`
      (`self.K2_DestroyActor`))))

(event `self.Target.OnComponentHit`
  (params (HitComponent :type "PrimitiveComponent Object Reference") (OtherActor :type "Actor Object Reference") (OtherComp :type "PrimitiveComponent Object Reference") (NormalImpulse :type "Vector Structure") (Hit :type "HitResult Structure (by ref)"))
  (cast `/Game/BPs/BP_FireSpell` OtherActor)
  (`self.Destroy`))

(fn `UserConstructionScript`)