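; BP_SplinePlatform is a platform actor that moves along the spline of a referenced SplineActor.
; On BeginPlay it sets a Timeline's play rate from Speed and plays it.
; Each Timeline update scales the track value by spline length and sets the Pivot component's world location and rotation to that point on the spline.
; Tick and the construction script are empty, and a few leftover nodes are unconnected.
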(event `self.ReceiveTick`
  (params (DeltaSeconds :type "Float (single-precision)")))

(event `self.ReceiveBeginPlay`
  (bind _spline (`/Game/BPs/BP_SplineActor.Spline` (`self.SplineActor`)))
  (`TimelineComponent.SetPlayRate` (`self.Timeline`) (`self.Speed`))
  (bind (_direction _newtrack_1) (`Timeline|Timeline`)
    (:`Update`
      (bind _returnvalue (* _newtrack_1 (`SplineComponent.GetSplineLength` _spline)))
      (`SceneComponent.K2_SetWorldLocation` (`self.pivot`) (`SplineComponent.GetLocationAtDistanceAlongSpline` _spline _returnvalue "World") false false)
      (`SceneComponent.K2_SetWorldRotation` (`self.pivot`) (`SplineComponent.GetRotationAtDistanceAlongSpline` _spline _returnvalue "World") false false))))

(fn `UserConstructionScript`)