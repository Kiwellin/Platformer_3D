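; Spline platform Blueprint that, by its name, is an improved variant of a platform placed along a spline.
; SetStartOffset converts StartOffset into DistanceAlongSpline by multiplying it by the length of the referenced SplineActor's spline.
; The construction script only calls its parent, and the event graph holds just disabled placeholder events, so this file contains no movement logic.
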(fn `SetStartOffset`
  (set `self.DistanceAlongSpline` (* (`self.StartOffset`) (`SplineComponent.GetSplineLength` (`/Game/BPs/BP_SplineActor.Spline` (`self.SplineActor`))))))

(fn `UserConstructionScript`
  (`parent.UserConstructionScript`))