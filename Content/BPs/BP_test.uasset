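; BP_test is a test actor that prints values from a small hardcoded float array every frame.
; BeginPlay fills the array, and Tick advances a float counter, truncates it to an index and prints that element.
; The counter resets only after equalling the array length, so it reads one past the last element each cycle.
; The Hit event and construction script are empty.
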(event `self.ReceiveTick`
  (params (DeltaSeconds :type "Float (single-precision)"))
  (if (== (`self.NewVar_0`) (`KismetArrayLibrary.Array_Length` (`self.NewVar`)))
    (set `self.NewVar_0` 0.0)
    (else
      (set `self.NewVar_0` (+ (`self.NewVar_0`) 1.0))))
  (`KismetSystemLibrary.PrintString` (`KismetStringLibrary.Conv_DoubleToString` (`|GetArrayItem` (`self.NewVar`) (`KismetMathLibrary.FTrunc` (`self.NewVar_0`))))))

(event `self.ReceiveBeginPlay`
  (set `self.NewVar` (`|MakeArray` 1.0 2.0 3.0 4.0)))

(event `self.ReceiveHit`
  (params (MyComp :type "PrimitiveComponent Object Reference") (Other :type "Actor Object Reference") (OtherComp :type "PrimitiveComponent Object Reference") (bSelfMoved :type Boolean) (HitLocation :type "Vector Structure") (HitNormal :type "Vector Structure") (NormalImpulse :type "Vector Structure") (Hit :type "HitResult Structure (by ref)")))

(fn `UserConstructionScript`)