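; BP_Worm is a stationary-style worm enemy that turns toward the player, attacks at close range and knocks the player back on overlap.
; Each tick it rotates on yaw only, with an animation curve slowing the turn toward near zero.
; Within range it plays an attack montage, re-armed by a DoOnce after montage length plus a pause.
; Overlap launches the character away and upward, throttled by a second DoOnce cooldown.
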(event `self.ReceiveBeginPlay`
  (bind _asbp_third_person_character (cast `/Game/BPs/BP_ThirdPersonCharacter` (`GameplayStatics.GetPlayerPawn` 0)))
  (set `self.Player` _asbp_third_person_character))

(event `self.ReceiveTick`
  (params (DeltaSeconds :type "Float (single-precision)"))
  (`self.LookAtPlayer`)
  (if (`self.IsInAttackrange`)
    (`/Engine/EditorBlueprintResources/StandardMacros.DoOnce` false :!label _label
      (:`Completed`
        (bind _montagelength (`self.Attack`))
        (`KismetSystemLibrary.Delay` (+ _montagelength (`self.TimeBetweenAttacks`)))
        (`self.Re-enable Attack`)))))

(event `Re-enable Attack`
  (goto _label :!via `Reset`))

(event `self.ReceiveActorBeginOverlap`
  (params (OtherActor :type "Actor Object Reference"))
  (bind (_returnvalue_x _returnvalue_y) (`KismetMathLibrary.BreakVector` (- (`self.K2_GetActorLocation` (`self.Player`)) (`self.K2_GetActorLocation`))))
  (bind _asbp_third_person_character (cast `/Game/BPs/BP_ThirdPersonCharacter` OtherActor))
  (`/Engine/EditorBlueprintResources/StandardMacros.DoOnce` false :!label _label_2
    (:`Completed`
      (`Character.LaunchCharacter` _asbp_third_person_character (* (+ (`KismetMathLibrary.Normal` (`KismetMathLibrary.MakeVector` _returnvalue_x _returnvalue_y)) (`KismetMathLibrary.MakeVector` 0.0 0.0 (`self.Knockback Z mutiplier`))) (`self.Knockback Strength`)) false false)
      (`KismetSystemLibrary.Delay` (`self.min delay between knockbacks`))
      (`self.Reset Knockback`))))

(event `Reset Knockback`
  (goto _label_2 :!via `Reset`))

(fn `Attack`
  (returns (MontageLength :type "Float (single-precision)"))
  (bind _returnvalue (`AnimInstance.Montage_Play` (`SkeletalMeshComponent.GetAnimInstance` (`self.SK_Worm`)) "/Game/Worm/Worm_Attack_Montage.Worm_Attack_Montage" 1.0 "MontageLength" 0.0 true))
  (return _returnvalue))

(fn `IsInAttackrange`
  (returns (ReturnValue :type Boolean))
  (return (<= (`KismetMathLibrary.VSize` (- (`self.K2_GetActorLocation`) (`self.K2_GetActorLocation` (`self.Player`)))) (`self.Distance to Worm`))))

(fn `LookAtPlayer`
  (bind (_returnvalue_roll _returnvalue_pitch _returnvalue_yaw) (`KismetMathLibrary.BreakRotator` (`KismetMathLibrary.FindLookAtRotation` (`self.K2_GetActorLocation`) (`self.K2_GetActorLocation` (`self.Player`)))))
  (`self.K2_SetActorRotation` (`KismetMathLibrary.RInterpTo_Constant` (`self.K2_GetActorRotation`) (`KismetMathLibrary.MakeRotator` 0.0 0.0 _returnvalue_yaw) (`GameplayStatics.GetWorldDeltaSeconds`) (`KismetMathLibrary.Lerp` (`self.MaxRotationSpeed`) 0.0001 (`AnimInstance.GetCurveValue` (`SkeletalMeshComponent.GetAnimInstance` (`self.SK_Worm`)) "RotationRestrictionPercentage")))))

(fn `UserConstructionScript`)